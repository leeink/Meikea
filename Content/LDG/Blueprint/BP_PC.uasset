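; Player controller for cursor-driven placement of actors picked by index from a class list.
; On BeginPlay it adds the input mapping, spawns a preview actor and shows the basic UI widget.
; While selection is active, Tick moves the preview to a cursor trace hit, raised slightly.
; Left click spawns another copy there and ends selection; setter functions change the index, selection state and preview, without destroying previous previews.
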(event `self.ReceiveBeginPlay`
  (`|ExecutionSequence`
    (:`then_0`
      (`EnhancedInputSubsystemInterface.AddMappingContext` (subsystem `EnhancedInputLocalPlayerSubsystem`) "/Game/LDG/Input/IMC_DefaultMappingContext.IMC_DefaultMappingContext" 0 (struct))
      (bind _returnvalue (`|SpawnActorFromClass` (`|GetArrayItem` (`self.SpawnActorClasses`) (`self.SelectIndex`)) (`KismetMathLibrary.MakeTransform` (0.0 0.0 0.0)) "Undefined" "MultiplyWithRoot" null null))
      (set `self.SelectActor` _returnvalue))
    (:`then_1`
      (bind _returnvalue_2 (`|CreateWidget` "/Game/Jin/Jin_Widget/Jin_UI/WBP_BasicUI.WBP_BasicUI_C"))
      (`UserWidget.AddToViewport` _returnvalue_2 0)
      (`WidgetBlueprintLibrary.SetInputMode_GameAndUIEx` self null))))

(event `self.ReceiveTick`
  (params (DeltaSeconds :type "Float (single-precision)"))
  (bind (_hitresult _returnvalue) (`self.GetHitResultUnderCursorByChannel` "TraceTypeQuery1"))
  (if (and (`self.bIsSelect`) _returnvalue)
    (bind _output_get (set `self.CursorLocation` (`.Location` (`GameplayStatics.BreakHitResult` _hitresult))))
    (`self.K2_SetActorLocation` (`self.SelectActor`) (+ _output_get (0.0 0.0 50.0)) false false)))

(event `EnhancedInput|/Game/LDG/Input/Actions/IA_MouseLeftClick`
  (params (ActionValue :type Boolean) (ElapsedSeconds :type "Float (double-precision)") (TriggeredSeconds :type "Float (double-precision)") (InputAction :type "InputAction Object Reference" :default "/Game/LDG/Input/Actions/IA_MouseLeftClick.IA_MouseLeftClick"))
  (:`Started`
    (`|SpawnActorFromClass` (`|GetArrayItem` (`self.SpawnActorClasses`) (`self.SelectIndex`)) (`KismetMathLibrary.MakeTransform` (+ (`self.CursorLocation`) (0.0 0.0 50.0))) "Undefined" "MultiplyWithRoot" null null)
    (`self.SetIsSelect` false)))

(fn `SetIsSelect`
  (params (NewParam :type Boolean))
  (set `self.bIsSelect` NewParam))

(fn `SetSelectActor`
  (set `self.SelectActor` null)
  (bind _returnvalue (`|SpawnActorFromClass` (`|GetArrayItem` (`self.SpawnActorClasses`) (`self.SelectIndex`)) (`KismetMathLibrary.MakeTransform` (+ (`self.CursorLocation`) (0.0 0.0 50.0))) "Undefined" "MultiplyWithRoot" null null))
  (set `self.SelectActor` _returnvalue))

(fn `SetSelectIndex`
  (params (NewIndex :type Integer))
  (set `self.SelectIndex` NewIndex))

(fn `UserConstructionScript`)